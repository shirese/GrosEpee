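; BP_Pickup_Mushroom is a mushroom collectible that is picked up when a BP_Sword overlaps its sphere.
; On BeginPlay it randomizes scale and yaw, plays audio pitched lower for larger mushrooms, and registers with BP_CaptureGameMode's pickup goal.
; On sword overlap it disables sphere collision, notifies the game mode, plays a pickup sound and destroys itself.
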(event `self.Sphere.OnComponentBeginOverlap`
  (params (OverlappedComponent :type "PrimitiveComponent Object Reference") (OtherActor :type "Actor Object Reference") (OtherComp :type "PrimitiveComponent Object Reference") (OtherBodyIndex :type Integer) (bFromSweep :type Boolean) (SweepResult :type "HitResult Structure (by ref)"))
  (cast `/Game/GameLogic/Blueprints/BP_Sword` OtherActor)
  (`PrimitiveComponent.SetCollisionEnabled` (`self.Sphere`) "NoCollision")
  (`/Game/GameLogic/Blueprints/BP_CaptureGameMode.OnPickup` (`self.CurrCaptureGameMode`))
  (`GameplayStatics.PlaySoundAtLocation` "/Game/Sounds/Pickup.Pickup" (`self.K2_GetActorLocation`) (struct) 1.0 1.0 0.0 null null null null)
  (`self.K2_DestroyActor`))

(event `self.ReceiveBeginPlay`
  (bind _output_get (set `self.MushroomScaleFactor` (`KismetMathLibrary.Conv_DoubleToVector` (+ (`KismetMathLibrary.RandomFloat`) 0.7))))
  (`AudioComponent.SetPitchMultiplier` (`self.Audio`) (`KismetMathLibrary.Lerp` 1.3 0.7 (.z _output_get)))
  (`AudioComponent.Play` (`self.Audio`) 0.0)
  (bind _asbp_capture_game_mode (cast `/Game/GameLogic/Blueprints/BP_CaptureGameMode` (`GameplayStatics.GetGameMode`)))
  (bind _output_get_2 (set `self.CurrCaptureGameMode` _asbp_capture_game_mode))
  (`/Game/GameLogic/Blueprints/BP_CaptureGameMode.IncrementPickupGoal` _output_get_2)
  (`self.SetActorScale3D` (`self.MushroomScaleFactor`))
  (`self.K2_SetActorRotation` (`KismetMathLibrary.MakeRotator` 0.0 0.0 (* (`KismetMathLibrary.RandomFloat`) 360.0))))

(fn `UserConstructionScript`)