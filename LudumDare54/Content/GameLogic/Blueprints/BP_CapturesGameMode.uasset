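; Game mode for a pickup game that creates the UI, spawns objects in a random-point box, and tracks pickups and destroyables.
; Tick drives spawning through Delays, with the respawn interval eased over elapsed game time.
; Health falls with outstanding spawns and destroyed count, adjusting ambient pitch and player walk speed.
; Zero health shows defeat in slow motion; the victory screen call is unconnected.
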(event `LooseEvent`
  (set `Widget.Visibility` "Visible" (`self.UI Defeat`))
  (`GameplayStatics.SetGlobalTimeDilation` 0.3))

(event `OnDestroy`
  ;[0.04688 0.04688 0.04688] LOOSE
  (bind _pickup_count (`self.AddDestroyable`))
  (`/Engine/EditorBlueprintResources/StandardMacros.CompareFloat` (/ (`KismetMathLibrary.Conv_IntToDouble` _pickup_count) (`self.DestroyableTotal`)) 0.6))

(event `AddHealth`
  (params (AddHealthVal :type "Float (double-precision)"))
  (set `self.Health` (`KismetMathLibrary.FMin` (+ (`self.Health`) AddHealthVal) 1.0)))

(event `UpdateGoal`
  ;[0.009375 0.009375 0.009375] Pickup
  (set `self.SpawnCountTarget` (+ (`self.SpawnCountTarget`) 1)))

(event `OnPickup`
  ;[0.009375 0.009375 0.009375] Pickup
  (set `self.SpawnCount` (+ (`self.SpawnCount`) -1))
  (bind _pickup_count (`self.AddPickupScore`))
  (`/Game/UI/UI_Overlay.SetObjectiveCounterText` (`self.UI Overlay`) (`self.PickupCount`))
  (if (>= _pickup_count (`self.PickupGoal`))
    (`self.UpdateGoal`)))

(event `UpdateHealth`
  (bind _audiocomponent (`AmbientSound.AudioComponent` (`self.Ambient`)))
  (bind _output_get (set `self.Health` (- 1.0 (+ (* (/ (`self.SpawnCount`) (`self.LooseSpawnCount`)) 0.4) (* (`KismetMathLibrary.FMin` (/ (`self.DestroyableCount`) (`KismetMathLibrary.Conv_IntToDouble` (/ (`self.DestroyableTotal`) 3.6))) 1.0) 0.6)))))
  (if (<= _output_get 0.0)
    (`AudioComponent.SetPitchMultiplier` _audiocomponent 0.24)
    (`self.LooseEvent`)
    (else
      (if (<= (mod _output_get 0.25) 0.05)
        (`AudioComponent.SetPitchMultiplier` _audiocomponent (+ (- 1.0 _output_get) 1.0)))
      (bind _output_get_2 (set `CharacterMovementComponent.MaxWalkSpeed` (* (`self.BaseWalkSpeed`) (+ (* (- 1.0 (`self.Health`)) (`self.TMP`)) 1.0)) (`Character.CharacterMovement` (`GameplayStatics.GetPlayerCharacter` 0)))))))

(event `UpdateTImeElapsed`
  (bind _maxgametime (`self.MaxGameTime`))
  (set `self.TimeElapsedDelta` (/ (`KismetMathLibrary.FMin` (`KismetSystemLibrary.GetGameTimeInSeconds`) _maxgametime) _maxgametime)))

(event `self.ReceiveTick`
  (params (DeltaSeconds :type "Float (single-precision)"))
  ;[0.03438 0.03438 0.03438] Time
  (`self.UpdateTImeElapsed`)
  (`self.UpdateRespawnDuration`)
  (`self.UpdateGoal`)
  (`self.UpdateHealth`)
  (`KismetSystemLibrary.Delay` (`self.Respawn Duration`))
  (if (< (`self.PickupGoal`) (`self.SpawnCountTarget`))
    (`KismetSystemLibrary.Delay` (`KismetMathLibrary.RandomFloatInRange` 0.0 (- 1.0 (`self.TimeElapsedDelta`))))
    (`/Game/GameLogic/Blueprints/BP_RandomPointInBox.SpawnBox` (`self.SpawnBox`))
    (set `self.SpawnCount` (+ (`self.SpawnCount`) 1))))

(event `UpdateRespawnDuration`
  (set `self.Respawn Duration` (`|EaseFunction` "EaseOut" (`self.TimeElapsedDelta`) (`self.BaseRespawnDuration`) (`self.EndRespawnDuration`) 4.0)))

(event `self.ReceiveBeginPlay`
  ;[0 0 0] Init
  (bind _returnvalue (`|CreateWidget` "/Game/UI/UI_VictoryScreen.UI_VictoryScreen_C"))
  (bind _output_get (set `self.VictoryScreenWidget` _returnvalue))
  (`UserWidget.AddToViewport` _output_get 0)
  (bind _returnvalue_2 (`|CreateWidget` "/Game/UI/UI_Overlay.UI_Overlay_C"))
  (bind _output_get_2 (set `self.UI Overlay` _returnvalue_2))
  (`UserWidget.AddToViewport` _output_get_2 0)
  (bind _returnvalue_3 (`|CreateWidget` "/Game/UI/UI_DefeatScreen.UI_DefeatScreen_C"))
  (bind _output_get_3 (set `self.UI Defeat` _returnvalue_3))
  (`UserWidget.AddToViewport` _output_get_3 0)
  (bind _returnvalue_4 (`GameplayStatics.GetActorOfClass` "/Game/GameLogic/Blueprints/BP_RandomPointInBox.BP_RandomPointInBox_C"))
  (set `self.SpawnBox` _returnvalue_4)
  (bind _returnvalue_5 (`|CreateWidget` "/Game/UI/UI_Health.UI_Health_C"))
  (`UserWidget.AddToViewport` _returnvalue_5 0)
  (bind _returnvalue_6 (`|CreateWidget` "/Game/UI/UI_Controls.UI_Controls_C"))
  (`UserWidget.AddToViewport` _returnvalue_6 -5)
  (bind _returnvalue_7 (`GameplayStatics.GetActorOfClass` "/Script/Engine.AmbientSound"))
  (set `self.Ambient` _returnvalue_7)
  (set `self.BaseWalkSpeed` (`CharacterMovementComponent.MaxWalkSpeed` (`Character.CharacterMovement` (`GameplayStatics.GetPlayerCharacter` 0)))))

(fn `AddDestroyable`
  (returns (`Pickup Count` :type Integer))
  (bind _output_get (set `self.DestroyableCount` (+ 1 (`self.DestroyableCount`))))
  (return _output_get))

(fn `AddDestroyableTotal`
  (returns (Total :type Integer))
  (bind _output_get (set `self.DestroyableTotal` (+ 1 (`self.DestroyableTotal`))))
  (return _output_get))

(fn `AddPickupScore`
  (returns (`Pickup Count` :type Integer))
  (bind _output_get (set `self.PickupCount` (+ 1 (`self.PickupCount`))))
  (return _output_get))

(fn `IncrementPickupGoal`
  (returns (PickupGoal :type Integer))
  (bind _output_get (set `self.PickupGoal` (+ 1.0 (`self.PickupGoal`))))
  (return _output_get))

(fn `IncrementPickupGoalRandom`
  (returns (PickupGoal :type Integer))
  (bind _output_get (set `self.PickupGoal` (+ (`KismetMathLibrary.RandomIntegerInRange` 5 15) (`self.PickupGoal`))))
  (return _output_get))

(fn `UserConstructionScript`)