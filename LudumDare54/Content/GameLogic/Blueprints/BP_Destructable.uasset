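; Destructible tree that loses a hit point (PV) each time a BP_Sword hits it and counts toward the captures game mode's destroyable total.
; A surviving hit spawns leaf particles, plays a chop sound and starts a brief shake, which Tick drives by lerping the capsule toward random pitch and roll.
; At zero PV it disables collision, notifies the game mode, plays a final sound and destroys its components, leaving the actor.
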(event `self.ReceiveTick`
  (params (DeltaSeconds :type "Float (single-precision)"))
  (bind _shaketime (`self.ShakeTime`))
  (bind _capsule (`self.Capsule`))
  (`/Engine/EditorBlueprintResources/StandardMacros.CompareFloat` _shaketime
    (:`>`
      (set `self.ShakeTime` (- _shaketime DeltaSeconds))
      (if (`KismetSystemLibrary.IsValid` _capsule)
        (`SceneComponent.K2_SetWorldRotation` _capsule (`KismetMathLibrary.RLerp` (`SceneComponent.K2_GetComponentRotation` _capsule) (`KismetMathLibrary.MakeRotator` (.x (* (* (`KismetMathLibrary.RandomUnitVector`) 360.0) (0.2 0.2 1.0))) (.y (* (* (`KismetMathLibrary.RandomUnitVector`) 360.0) (0.2 0.2 1.0))) (.yaw (`SceneComponent.K2_GetComponentRotation` _capsule))) 0.05) false false)))))

(event `self.ReceiveHit`
  (params (MyComp :type "PrimitiveComponent Object Reference") (Other :type "Actor Object Reference") (OtherComp :type "PrimitiveComponent Object Reference") (bSelfMoved :type Boolean) (HitLocation :type "Vector Structure") (HitNormal :type "Vector Structure") (NormalImpulse :type "Vector Structure") (Hit :type "HitResult Structure (by ref)"))
  (cast `/Game/GameLogic/Blueprints/BP_Sword` Other)
  (`KismetSystemLibrary.PrintString` "Tree HITTED")
  (bind _output_get (set `self.PV` (- (`self.PV`) 1)))
  (`/Engine/EditorBlueprintResources/StandardMacros.CompareInt` _output_get
    (:`>`
      (`SceneComponent.K2_SetWorldRotation` :`self` (`self.Capsule`))
      (`NiagaraFunctionLibrary.SpawnSystemAtLocation` "/Game/Art/VFX/NS_Leaves.NS_Leaves" (+ (`SceneComponent.K2_GetComponentLocation` (`self.Cylinder`)) (0.0 0.0 150.0)))
      (set `self.ShakeTime` 0.3)
      (`GameplayStatics.PlaySoundAtLocation` "/Game/Sounds/chopWood.chopWood" (`self.K2_GetActorLocation`) (struct) 1.0 1.0 0.0 null null null null))
    (:`==`
      (`PrimitiveComponent.SetCollisionEnabled` (`self.Capsule`) "NoCollision" :!label _label)
      (`/Game/GameLogic/Blueprints/BP_CapturesGameMode.OnDestroy` (`self.CurrCaptureGameMode`))
      (`GameplayStatics.PlaySoundAtLocation` "/Game/Sounds/chopWood1.chopWood1" (`self.K2_GetActorLocation`) (struct) 1.0 1.0 0.0 null null null null)
      (`ActorComponent.K2_DestroyComponent` (`self.Capsule`))
      (`ActorComponent.K2_DestroyComponent` (`self.Cylinder`)))
    (:`<`
      (goto _label))))

(event `self.ReceiveBeginPlay`
  (bind _asbp_captures_game_mode (cast `/Game/GameLogic/Blueprints/BP_CapturesGameMode` (`GameplayStatics.GetGameMode`)))
  (bind _output_get (set `self.CurrCaptureGameMode` _asbp_captures_game_mode))
  (`/Game/GameLogic/Blueprints/BP_CapturesGameMode.AddDestroyableTotal` _output_get))

(fn `UserConstructionScript`)