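; Thrown sword actor that flies as a spinning physics sphere for a set air time, with SetState toggling its visibility and collision.
; Throw launches it horizontally; Tick then re-normalizes velocity to constant speed and spin until the timer expires, when movement stops and spin decays.
; The timer and physics updates pause under slow time dilation, which also silences the staged spin sound.
; BeginPlay attaches a Niagara trail sized between two blade sockets.
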(event `self.ReceiveTick`
  (params (DeltaSeconds :type "Float (single-precision)"))
  (bind _sphere_col (`self.Sphere_Col`))
  (`/Engine/EditorBlueprintResources/StandardMacros.CompareFloat` (`GameplayStatics.GetGlobalTimeDilation`) 0.8
    (:`>`
      (bind _output_get (set `self.RotTImer` (- (`self.RotTImer`) DeltaSeconds)))
      (`/Engine/EditorBlueprintResources/StandardMacros.CompareFloat` _output_get
        (:`>`
          (`self.Activate Spinning Sound`)
          (bind _returnvalue (`PrimitiveComponent.GetPhysicsLinearVelocity` _sphere_col "None"))
          (`PrimitiveComponent.SetAllPhysicsLinearVelocity` _sphere_col (* (`KismetMathLibrary.Normal` _returnvalue) (`self.Speed`)) false)
          (`PrimitiveComponent.SetPhysicsAngularVelocityInDegrees` _sphere_col (`KismetMathLibrary.MakeVector` 0.0 0.0 (`self.AngularSpeed`)) false "None"))
        (:`<`
          (`self.Deactivate Spinning Sound`)
          (`PrimitiveComponent.SetAllPhysicsLinearVelocity` _sphere_col (0.0 0.0 0.0) false)
          (`PrimitiveComponent.SetPhysicsAngularVelocityInDegrees` _sphere_col (* (`PrimitiveComponent.GetPhysicsAngularVelocityInDegrees` _sphere_col "None") (`KismetMathLibrary.Conv_DoubleToVector` 0.95)) false "None"))))
    (:`<`
      (`self.Deactivate Spinning Sound`))))

(event `self.ReceiveBeginPlay`
  (bind _mdl_grosepee (`self.mdl_grosEpee`))
  (bind _returnvalue (`SceneComponent.GetSocketLocation` _mdl_grosepee "Trail_Top"))
  (bind _returnvalue_2 (`SceneComponent.GetSocketLocation` _mdl_grosepee "Trail_Bottom"))
  (bind _returnvalue_3 (- _returnvalue _returnvalue_2))
  (`AudioComponent.SetSound` (`self.sfx_grosEpee`) (`self.SpinSound`))
  (bind _returnvalue_4 (`NiagaraFunctionLibrary.SpawnSystemAttached` "/Game/Art/VFX/NS_SwordTrails.NS_SwordTrails" _mdl_grosepee "None" (/ (+ _returnvalue _returnvalue_2) 2.0) (`KismetMathLibrary.MakeRotFromZ` _returnvalue_3) "KeepWorldPosition"))
  (`FXSystemComponent.SetFloatParameter` _returnvalue_4 "TrailWidth" (`KismetMathLibrary.VSize` _returnvalue_3)))

(event `Activate Spinning Sound`
  ;[1 1 1] Sound
  (if (not (`self.IsSpinning`))
    (set `self.IsSpinning` true)
    (`AudioComponent.Play` (`self.sfx_grosEpee`) 0.0)
    (`KismetSystemLibrary.Delay` 0.6125)
    (`AudioComponent.Play` (`self.sfx_grosEpee`) 0.0)
    (`KismetSystemLibrary.Delay` 0.6125)
    (`AudioComponent.Play` (`self.sfx_grosEpee`) 6.1)))

(event `Deactivate Spinning Sound`
  ;[1 1 1] Sound
  (if (`self.IsSpinning`)
    (set `self.IsSpinning` false)
    (`AudioComponent.Stop` (`self.sfx_grosEpee`))))

(fn `SetCollisions`
  (params (state :type Boolean))
  (bind _sphere_col (`self.Sphere_Col`))
  (if state
    (`PrimitiveComponent.SetCollisionEnabled` _sphere_col "QueryAndPhysics")
    (else
      (`PrimitiveComponent.SetCollisionEnabled` _sphere_col "NoCollision"))))

(fn `SetHidden`
  (params (value :type Boolean))
  (`SceneComponent.SetHiddenInGame` (`self.Sphere_Col`) value true))

(fn `SetState`
  (params (state :type Boolean))
  (`self.SetHidden` (not state))
  (`self.SetCollisions` state))

(fn `Throw`
  (params (dir :type "Vector Structure"))
  (bind _sphere_col (`self.Sphere_Col`))
  (`PrimitiveComponent.SetSimulatePhysics` _sphere_col true)
  (`PrimitiveComponent.SetAllPhysicsLinearVelocity` _sphere_col (* (`KismetMathLibrary.Normal` (`KismetMathLibrary.MakeVector` (.x dir) (.y dir))) (`self.Speed`)) false)
  (`PrimitiveComponent.SetPhysicsAngularVelocityInDegrees` _sphere_col (`KismetMathLibrary.MakeVector` 0.0 0.0 (`self.AngularSpeed`)) false "None")
  (set `self.RotTImer` (`self.AirTime`)))

(fn `UserConstructionScript`)